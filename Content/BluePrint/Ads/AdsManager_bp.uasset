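; Rewarded-video ad manager that grants skill, balloon skill or medal rewards through several ad networks.
; On BeginPlay it sets up each enabled network among Unity Ads, AdColony, AppLovin and Chartboost; Vungle is left disconnected.
; WatchAds shows the first available video in fixed priority order, with preloading for AppLovin and Chartboost.
; Each request stores its reward type, and completion callbacks or a NoAds bypass pass it to CallFinishedWatching.
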(event DidAppLovinfailedtoReceiveAd(AppLovin)
  (Class|AppLovinFunctions|AppLovinPreloadRewardedVideo))

(event DidFailtoLoadRewardedVideo(Chartboost)
  (params (Location :type String))
  (Class|ChartboostFunctions|ChartboostCacheRewardedVideo (Variables|Default|GetChartBoostVideoReward)))

(event DidCloseRewardedVideo(Chartboost)
  (params (Location :type String))
  (Class|ChartboostFunctions|ChartboostCacheRewardedVideo (Variables|Default|GetChartBoostVideoReward)))

(event DidCompleteRewardedVideo(Chartboost)
  (params (Location :type String) (Reward :type Integer))
  (Class|ChartboostFunctions|ChartboostCacheRewardedVideo (Variables|Default|GetChartBoostVideoReward))
  (CallFunction|OnFinishedWatching))

(event EventBeginPlay
  (Utilities|FlowControl|Sequence
    (:then_0
      (if (Variables|Default|GetUseUnityAds)
        (CallFunction|ConstructUnityAds)))
    (:then_1
      (if (Variables|Default|GetUseAdColony)
        (CallFunction|ConstructAdColony)))
    (:then_2
      (if (Variables|Default|GetUseAppLovin)
        (CallFunction|ConstructAppLovin)))
    (:then_3
      (if (Variables|Default|GetUseChartboost)
        (CallFunction|ConstructChartBoost)))))

(fn ConstructionScript)

(fn ConstructChartBoost
  (Class|ChartboostFunctions|ChartboostCacheRewardedVideo (Variables|Default|GetChartBoostVideoReward))
  (EventDispatchers|BindEventtoDidCompleteRewardedVideo (Variables|Default|GetChartboost) (EventDispatchers|CreateEvent :!event OnChartboostFinishWatching)))

(fn WatchAds
  (Utilities|FlowControl|Sequence
    (:then_0
      (if (Class|UnityAdsFunctions|UnityAdsHasRewardedVideo)
        (Class|UnityAdsFunctions|UnityAdsShowRewardedVideo)
        (return true)))
    (:then_1
      (if (Class|AppLovinFunctions|AppLovinHasRewardedVideo)
        (Class|AppLovinFunctions|AppLovinShowRewardedVideo)
        (Class|AppLovinFunctions|AppLovinPreloadRewardedVideo)
        (return true)))
    (:then_2
      (if (Class|ChartboostFunctions|ChartboostHasRewardedVideo "Default")
        (Class|ChartboostFunctions|ChartboostShowRewardedVideo (Variables|Default|GetChartBoostVideoReward))
        (return true)))
    (:then_3
      (if (Variables|Default|GetAdColonyAvailability)
        (Class|AdColonyFunctions|AdColonyShowV4VCReward)
        (return true)))
    (:then_4
      (if (Class|ChartboostFunctions|ChartboostHasRewardedVideo (Variables|Default|GetChartBoostVideoReward))
        (Class|ChartboostFunctions|ChartboostShowRewardedVideo (Variables|Default|GetChartBoostVideoReward))
        (Class|ChartboostFunctions|ChartboostCacheRewardedVideo (Variables|Default|GetChartBoostVideoReward))
        (return true)))
    (:then_5
      (return false))))

(fn ConstructUnityAds
  (EventDispatchers|BindEventtoOnUnityAdsReady (Variables|Default|GetUnityAds) (EventDispatchers|CreateEvent :!event OnUnityAdsReady))
  (EventDispatchers|BindEventtoOnUnityAdsFinish (Variables|Default|GetUnityAds) (EventDispatchers|CreateEvent :!event OnFinishedWatching)))

(fn ConstructAdColony
  (EventDispatchers|BindEventtoDidAdColonyAdAvailabilityChange (Variables|Default|GetAdColony) (EventDispatchers|CreateEvent :!event OnAdColonyStatusChange))
  (EventDispatchers|BindEventtoDidAdColonyCompleteRewardedVideo (Variables|Default|GetAdColony) (EventDispatchers|CreateEvent :!event OnAdColonyFinishedWatching)))

(fn ConstructAppLovin
  (EventDispatchers|BindEventtoDidAppLovinCompleteRewardedVideo (Variables|Default|GetAppLovin) (EventDispatchers|CreateEvent :!event OnFinishedWatching))
  (Class|AppLovinFunctions|AppLovinPreloadRewardedVideo))

(fn ConstructVungle)

(fn OnUnityAdsReady
  (Variables|Default|SetUnityAdsOK true))

(fn OnFinishedWatching
  (Default|CallFinishedWatching (Variables|Default|GetLastRewardRequest) (Variables|Default|GetLastActiveSkillRequest) (Variables|Default|GetLastActiveBalloonSkillRequest)))

(fn OnAdColonyStatusChange
  (params (Availability :type Boolean))
  (Variables|Default|SetAdColonyAvailability Availability))

(fn OnAdColonyFinishedWatching
  (params (Reward :type Integer))
  (CallFunction|OnFinishedWatching))

(fn OnVungleFinishedWatching
  (params (Successful :type Boolean))
  (if Successful
    (CallFunction|OnFinishedWatching)))

(fn OnChartboostFinishWatching
  (params (Message :type String) (Status :type Integer))
  (CallFunction|OnFinishedWatching))

(fn OnVungleStatusChange
  (params (Availability :type Boolean))
  (Development|PrintString (Utilities|String|Append "Vungle Available: " (Utilities|String|ToString(Boolean) Availability)) true true "(R=0.000000,G=0.660000,B=1.000000,A=1.000000)" 5.0))

(fn AdsAvailabilityStatus
  (return (Math|Boolean|ORBoolean (Class|UnityAdsFunctions|UnityAdsHasRewardedVideo) (Class|AppLovinFunctions|AppLovinHasRewardedVideo) (Variables|Default|GetAdColonyAvailability) (Class|ChartboostFunctions|ChartboostHasRewardedVideo "Default"))))

(fn WatchAdsActiveSkill
  (params (RequestSkill :type EActiveSkillType%20Enum) (NoAds :type Boolean))
  (Utilities|FlowControl|Sequence
    (:then_0
      (Variables|Default|SetLastActiveSkillRequest RequestSkill)
      (Variables|Default|SetLastRewardRequest "Skill"))
    (:then_1
      (if NoAds
        (CallFunction|OnFinishedWatching)
        (return true)
        (else
          (bind _success (CallFunction|WatchAds))
          (return _success))))))

(fn WatchAdsforBalloonSkill
  (params (BalloonSkill :type Balloon%20Skill%20Structure) (NoAds :type Boolean))
  (Utilities|FlowControl|Sequence
    (:then_0
      (Variables|Default|SetLastActiveBalloonSkillRequest BalloonSkill)
      (Variables|Default|SetLastRewardRequest "Ballon"))
    (:then_1
      (if NoAds
        (CallFunction|OnFinishedWatching)
        (return true)
        (else
          (bind _success (CallFunction|WatchAds))
          (return _success))))))

(fn WatchAdsforMedal
  (params (NoAds :type Boolean))
  (Utilities|FlowControl|Sequence
    (:then_0
      (Variables|Default|SetLastRewardRequest "Medal"))
    (:then_1
      (if NoAds
        (CallFunction|OnFinishedWatching)
        (return true)
        (else
          (bind _success (CallFunction|WatchAds))
          (return _success))))))