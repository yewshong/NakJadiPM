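; Balloon actor for a 2D Paper2D touch game that rises while bouncing side to side between X limits.
; Tick moves it by delta-scaled speeds, flips horizontal speed at the bounds and destroys it above a maximum height.
; A touch swaps the sprite for a one-shot flipbook animation.
; When the animation finishes, the actor destroys itself, then fires the BallonClicked dispatcher.
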(event OnInputTouchBegin(PaperSprite)
  (params (FingerIndex :type ETouchIndex%20Enum :default "Touch1") (TouchedComponent :type Primitive%20Component%20Object%20Reference))
  (CallFunction|UpdateBallonClick))

(event OnFinishedPlaying(PaperFlipbook)
  (Development|PrintString "done!")
  (Actor|DestroyActor)
  (Default|CallBallonClicked))

(event Custom|UpdateBallonClick
  (Rendering|SetVisibility (Variables|Default|GetPaperSprite) false false)
  (Rendering|SetVisibility (Variables|Default|GetPaperFlipbook) true false)
  (Components|Timeline|PlayfromStart (Variables|Default|GetPaperFlipbook))
  (Components|Timeline|SetLooping (Variables|Default|GetPaperFlipbook) false))

(event EventBeginPlay)

(event Collision|EventActorBeginOverlap
  (params (OtherActor :type Actor%20Object%20Reference)))

(event EventTick
  (params (DeltaSeconds :type Float%20%28single-precision%29))
  (CallFunction|DestroyActorifExceedHeight)
  (CallFunction|UpdateMovement))

(fn ConstructionScript)

(fn UpdateMovement
  (bind _returnvalue (Transformation|GetActorLocation))
  (bind _returnvalue_2 (Transformation|GetActorLocation))
  (Utilities|FlowControl|Sequence
    (:then_0
      (if (or (<= (.x _returnvalue_2) (Variables|Default|GetMinX)) (>= (.x _returnvalue_2) (Variables|Default|GetMaxX)))
        (Variables|Default|SetSpeedSide (* (Variables|Default|GetSpeedSide) -1.0))))
    (:then_1
      (Transformation|SetActorLocation (Math|Vector|MakeVector (+ (.x _returnvalue) (* (Utilities|Time|GetWorldDeltaSeconds) (Variables|Default|GetSpeedSide))) (.y _returnvalue) (+ (.z _returnvalue) (* (Utilities|Time|GetWorldDeltaSeconds) (Variables|Default|GetSpeedUp)))) false false))))

(fn DestroyActorifExceedHeight
  (if (>= (.z (Transformation|GetActorLocation)) (Variables|Default|GetMaxHeight))
    (Actor|DestroyActor)))