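; AchievementManager is an actor that reads, writes and displays the local player's platform achievements.
; On BeginPlay it caches achievements for player controller 0, then loops over AchievementIDs to append each cached progress value to AchievementProgress.
; Custom events write progress for a given ID and open the platform-specific achievements screen.
; Cache success or failure sets AchievementsCached and prints a debug message.
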(event Custom|WriteAchievementProgress
  (params (AchievementID :type Name) (Progress :type Float%20%28single-precision%29))
  (|WriteAchievementProgress (Game|GetPlayerController 0) AchievementID Progress))

(event Custom|ShowPlatformScreen
  (Class|KismetSystemLibrary|ShowPlatformSpecificAchievementsScreen (Game|GetPlayerController 0)))

(event EventBeginPlay
  (|CacheAchievements (Game|GetPlayerController 0)
    (:OnSuccess
      (Variables|Default|SetAchievementsCached true)
      (CallFunction|GetAchievementsProgress)
      (Development|PrintString "Read achievements Successfully" true true "(R=0.000000,G=0.660000,B=1.000000,A=1.000000)" 1e+01))
    (:OnFailure
      (Variables|Default|SetAchievementsCached false)
      (Development|PrintString "failed to read Achievements" true true "(R=0.000000,G=0.660000,B=1.000000,A=1.000000)" 1e+01))))

(event Collision|EventActorBeginOverlap
  (params (OtherActor :type Actor%20Object%20Reference)))

(event EventTick
  (params (DeltaSeconds :type Float%20%28single-precision%29)))

(fn ConstructionScript)

(fn GetAchievementsProgress
  (if (Variables|Default|GetAchievementsCached)
    (for _array_element (Variables|Default|GetAchievementIDs)
      (bind _progress (Class|AchievementBlueprintLibrary|GetCachedAchievementProgress (Game|GetPlayerController 0) _array_element))
      (Utilities|Array|Add (Variables|Default|GetAchievementProgress) _progress))))