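; LeaderboardManager is a Blueprint that reads, writes and displays a platform online leaderboard identified by its LeaderboardName variable.
; On BeginPlay it queries the first player's leaderboard value, storing it in LeaderBoardValue, setting GotRank and printing a debug message on success or failure.
; Separate events write an integer score to that leaderboard and open the platform-specific leaderboard screen.
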(event Custom|GetPlayerRank
  (bind _leaderboardvalue (|LeaderboardQuery (Game|GetPlayerController 0) (Variables|Default|GetLeaderboardName))
    (:OnSuccess
      (Variables|Default|SetGotRank true)
      (Variables|Default|SetLeaderBoardValue _leaderboardvalue)
      (Development|PrintString "Read leaderborad Successfully" true true "(R=0.000000,G=0.660000,B=1.000000,A=1.000000)" 1e+01))
    (:OnFailure
      (Variables|Default|SetGotRank false)
      (Development|PrintString "failed to read leaderborad" true true "(R=0.000000,G=0.660000,B=1.000000,A=1.000000)" 1e+01))))

(event Custom|WriteScoreLeaderBoard
  (params (Score :type Integer))
  (Class|LeaderboardBlueprintLibrary|WriteLeaderboardInteger (Game|GetPlayerController 0) (Variables|Default|GetLeaderboardName) Score))

(event Custom|ShowPlatformLeaderBoard
  (Class|KismetSystemLibrary|ShowPlatformSpecificLeaderboardScreen (Utilities|String|ToString(Name) (Variables|Default|GetLeaderboardName))))

(event EventBeginPlay
  (CallFunction|GetPlayerRank))

(fn ConstructionScript)