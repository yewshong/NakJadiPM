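; Blueprint function library that gives global access to the game's manager actors: sound, text, achievements, leaderboards, gameplay, Android IAP and ads.
; Each getter runs GetAllActorsOfClass on every call and returns the first result, assuming one placed instance with no validity check.
; GetSettings finds the GeneralDataManager the same way, creates player settings if none exist, and returns them through its SaveGameManager.
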(fn GetSoundPlayer
  (bind _outactors (Actor|GetAllActorsOfClass 0 "/Game/BluePrint/Sound/SoundPlayer_bp.SoundPlayer_bp_C"))
  (return (Utilities|Array|Get(acopy) _outactors)))

(fn GetTextManager
  (bind _outactors (Actor|GetAllActorsOfClass 0 "/Script/NakJadiPM.RetrieveTextManager"))
  (return (Utilities|Array|Get(acopy) _outactors)))

(fn GetAchievementManager
  (bind _outactors (Actor|GetAllActorsOfClass 0 "/Game/BluePrint/AchievementAndLeaderboard/AchievementManager.AchievementManager_C"))
  (return (Utilities|Array|Get(acopy) _outactors)))

(fn GetLeaderboardManager
  (bind _outactors (Actor|GetAllActorsOfClass 0 "/Game/BluePrint/AchievementAndLeaderboard/LeaderboardManager.LeaderboardManager_C"))
  (return (Utilities|Array|Get(acopy) _outactors)))

(fn GetGamePlayManager
  (bind _outactors (Actor|GetAllActorsOfClass 0 "/Script/NakJadiPM.GamePlayManager"))
  (return (Utilities|Array|Get(acopy) _outactors)))

(fn GetIAPManager
  (bind _outactors (Actor|GetAllActorsOfClass 0 "/Game/BluePrint/IAP/AndroidIAPManager.AndroidIAPManager_C"))
  (return (Utilities|Array|Get(acopy) _outactors)))

(fn GetAdsManager
  (bind _outactors (Actor|GetAllActorsOfClass 0 "/Game/BluePrint/Ads/AdsManager_bp.AdsManager_bp_C"))
  (return (Utilities|Array|Get(acopy) _outactors)))

(fn GetSettings
  (bind _outactors (Actor|GetAllActorsOfClass 0 "/Script/NakJadiPM.GeneralDataManager"))
  (bind _output_get (LocalVariables|SetGeneralDatamanager (Utilities|Array|Get(acopy) _outactors)))
  (bind _returnvalue (Class|GeneralDataManager|PlayerSettingsExists _output_get))
  (if _returnvalue
    _
    (else
      (Class|GeneralDataManager|CreateNewPlayerSettings (LocalVariables|GetGeneralDatamanager))))
  (bind _returnvalue_2 (Class|SaveGameManager|GetPlayerSettings (Variables|/Script/NakJadiPM.GeneralDataManager|GetSaveGameManager (LocalVariables|GetGeneralDatamanager))))
  (return _returnvalue_2))