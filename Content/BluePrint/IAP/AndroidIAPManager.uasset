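; Android in-app purchase manager that queries store products, makes purchases and restores past purchases.
; On BeginPlay it queries the product ID list and broadcasts the retrieved products.
; PurchaseProduct and RestorePurchase forward to events that run the async InAppPurchase and InAppPurchaseRestore nodes, broadcasting purchase success or failure and successful restores.
; On-screen debug prints trace queries and purchases, including each failure status.
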(event Custom|MakeRestore
  (params (Product :type Array%20of%20Product%20Data%20Structures))
  (Utilities|Array|Clear (Variables|Default|GetProductRequests))
  (for _array_element Product
    (Utilities|Array|Add (Variables|Default|GetProductRequests) (Utilities|Struct|MakeInAppPurchaseProductRequest (.ProductID (Utilities|Struct|BreakProductData _array_element)) (.Consumeable (Utilities|Struct|BreakProductData _array_element)))))
  (bind _inapprestorepurchaseinformation (|InAppPurchaseRestore (Variables|Default|GetProductRequests) (Game|GetPlayerController 0))
    (:OnSuccess
      (Default|CallProductsRestored _inapprestorepurchaseinformation))))

(event Custom|MakePurchase
  (params (Product :type Product%20Data%20Structure))
  (bind (_productid _consumeable) (Utilities|Struct|BreakProductData Product))
  (Development|PrintString (Utilities|String|Append "Trying to buy Product : " _productid " @ Consumeable" (Utilities|String|ToString(Boolean) _consumeable)) true true "(R=0.262638,G=1.000000,B=0.070987,A=1.000000)" 3e+02)
  (bind (_completionstatus _inapppurchaseinformation) (|InAppPurchase (Game|GetPlayerController 0) (Utilities|Struct|MakeInAppPurchaseProductRequest _productid _consumeable))
    (:OnSuccess
      (Default|CallProductPurchaseDone _inapppurchaseinformation _completionstatus)
      (Development|PrintString "Product bought" true true "(R=0.262638,G=1.000000,B=0.070987,A=1.000000)" 1e+02))
    (:OnFailure
      (Default|CallProductPurchaseFailed _inapppurchaseinformation _completionstatus)
      (switch Utilities|FlowControl|Switch|SwitchonEInAppPurchaseState _completionstatus
        (:Unknown
          (Development|PrintString "Failed to buy: unknown" true true "(R=0.262638,G=1.000000,B=0.070987,A=1.000000)" 1e+02))
        (:Success
          (Development|PrintString "Failed to buy: unknown" true true "(R=0.262638,G=1.000000,B=0.070987,A=1.000000)" 1e+02))
        (:Failed
          (Development|PrintString "Failed to buy: failed" true true "(R=0.262638,G=1.000000,B=0.070987,A=1.000000)" 1e+02))
        (:Cancelled
          (Development|PrintString "Failed to buy: Cancelled" true true "(R=0.262638,G=1.000000,B=0.070987,A=1.000000)" 1e+02))
        (:Invalid
          (Development|PrintString "Failed to buy: Invalid" true true "(R=0.262638,G=1.000000,B=0.070987,A=1.000000)" 1e+02))
        (:NotAllowed
          (Development|PrintString "Failed to buy: Not Allowed" true true "(R=0.262638,G=1.000000,B=0.070987,A=1.000000)" 1e+02))
        (:Restored
          (Development|PrintString "Failed to buy: Restored" true true "(R=0.262638,G=1.000000,B=0.070987,A=1.000000)" 1e+02))
        (:AlreadyOwned
          (Development|PrintString "Failed to buy: Already owned" true true "(R=0.262638,G=1.000000,B=0.070987,A=1.000000)" 1e+02))))))

(event EventBeginPlay
  (Development|PrintString "Starting to get producs" true true "(R=0.000000,G=0.660000,B=1.000000,A=1.000000)" 5e+03)
  (bind _inapppurchaseinformation (|InAppPurchaseQuery (Game|GetPlayerController 0) (Variables|Default|GetProductIDsList))
    (:OnSuccess
      (Default|CallProductsRetrieveDone _inapppurchaseinformation)
      (Development|PrintString "Products received" true true "(R=0.000000,G=0.660000,B=1.000000,A=1.000000)" 5e+03))
    (:OnFailure
      (Development|PrintString "Get products failed" true true "(R=0.000000,G=0.660000,B=1.000000,A=1.000000)" 5e+03))))

(event EventTick
  (params (DeltaSeconds :type Float%20%28single-precision%29)))

(fn ConstructionScript)

(fn RestorePurchase
  (params (Products :type Array%20of%20Product%20Data%20Structures))
  (CallFunction|MakeRestore Products))

(fn PurchaseProduct
  (params (Product :type Product%20Data%20Structure))
  (CallFunction|MakePurchase Product))