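; SoundPlayer_bp is an actor that plays UI and effect sounds such as taps, pops, button presses and coins.
; Each Play function starts an audio component from the beginning, with button click reusing the dialogue pop sound.
; MuteSound sets a volume multiplier to zero or full, which ProcessVolumes applies to every audio component on the actor.
; PlayEffectSound switches on an effect enum but plays nothing.
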(event EventBeginPlay)

(event Collision|EventActorBeginOverlap
  (params (OtherActor :type Actor%20Object%20Reference)))

(fn ConstructionScript)

(fn PlayTapSound
  (Audio|Components|Audio|Play (Variables|Default|GetTapAudio) 0.0))

(fn PlayBalloonPop
  (Audio|Components|Audio|Play (Variables|Default|GetBalloonPopAudio) 0.0))

(fn PlayDialoguePop
  (Audio|Components|Audio|Play (Variables|Default|GetDialoguePopAudio) 0.0))

(fn PlayButtonClick
  (Audio|Components|Audio|Play (Variables|Default|GetDialoguePopAudio) 0.0))

(fn PlayEffectSound
  (params (FXEnum :type EffectSoundEnum%20Enum))
  (switch Utilities|FlowControl|Switch|SwitchonEffectSoundEnum FXEnum))

(fn PlayButtonYes
  (Audio|Components|Audio|Play (Variables|Default|GetButtonYes) 0.0))

(fn PlayButtonNo
  (Audio|Components|Audio|Play (Variables|Default|GetButtonNo) 0.0))

(fn PlayCoin
  (Audio|Components|Audio|Play (Variables|Default|GetCoin) 0.0))

(fn MuteSound
  (params (Mute :type Boolean))
  (bind _output_get (Variables|Default|SetMute Mute))
  (if _output_get
    (Variables|Default|SetVolumeMultiplier 0.0)
    (else
      (Variables|Default|SetVolumeMultiplier 1.0)))
  (CallFunction|ProcessVolumes))

(fn ProcessVolumes
  (for _array_element (Actor|GetComponentsByClass "/Script/Engine.AudioComponent")
    (Audio|Components|Audio|SetVolumeMultiplier _array_element (Variables|Default|GetVolumeMultiplier) :!class /Script/Engine.AudioComponent)))