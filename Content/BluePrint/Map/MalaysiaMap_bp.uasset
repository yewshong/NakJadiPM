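; Malaysia map actor that highlights the state of the latest seat in the campaign's seat possession record and frames it.
; Tick polls GamePlayManager for state changes, then swaps in the highlight material and reapplies per-state colors.
; Three zoom levels (whole country, East/West half, single state) pick focus data loaded from a data table.
; The map actor itself lerps location and scale toward that target, rather than moving a camera.
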(event EventBeginPlay
  (CallFunction|AssignColortoStates)
  (bind _outactors (Actor|GetAllActorsOfClass "/Script/NakJadiPM.GamePlayManager"))
  (if (> (Utilities|Array|Length _outactors) 0)
    (Variables|Default|SetGamePlayManager (Utilities|Array|Get(acopy) _outactors))
    (Variables|Default|SetCurrentZoomLevel (Variables|Default|GetMaxZoom))
    (CallFunction|LoadMapFocusData)))

(event EventTick
  (params (DeltaSeconds :type Float%20%28single-precision%29))
  (bind _gameplaymanager (Variables|Default|GetGamePlayManager))
  (bind _currentgamedata (Variables|/Script/NakJadiPM.GamePlayManager|GetCurrentGameData _gameplaymanager))
  (bind _campaigndata (Variables|/Script/NakJadiPM.CampaignSaveGame|GetCampaignData _currentgamedata))
  (bind (_finished _finishedreported _achievement _starttime _endtime _lastsavedtime _lastprocesstime _selectedcandidate _selectedparty _timeremaining _balance _clickdamage _votespersecond _parlimentseatsdata _statesdata _skillscostdata _activeskilldata _candidatesdata _seatpossessionrecord) (Utilities|Struct|BreakCurrentCampaignData _campaigndata))
  (bind _parlimentseats (Utilities|Struct|BreakAllParlimentSeatsData _parlimentseatsdata))
  (bind _returnvalue (Utilities|Array|LastIndex _seatpossessionrecord))
  (bind _item (Utilities|Array|Get(acopy) _seatpossessionrecord _returnvalue))
  (bind _index (Utilities|Struct|BreakParlimentSeatResult _item))
  (bind _item_2 (Utilities|Array|Get(acopy) _parlimentseats _index))
  (bind _state (Utilities|Struct|BreakParlimentSeat _item_2))
  (if (!= (Variables|Default|GetGamePlayManager) 0)
    (if (!= (Variables|/Script/NakJadiPM.GamePlayManager|GetCurrentGameData (Variables|Default|GetGamePlayManager)) 0)
      (if (Utilities|Enum|NotEqual(Enum) _state (Variables|Default|GetCurrentState))
        (bind _output_get (Variables|Default|SetCurrentState _state))
        (CallFunction|SetActiveState _output_get)
        (CallFunction|UpdateZoom))
      (CallFunction|UpdateMapTransform))))

(fn ConstructionScript)

(fn AssignColortoStates
  (bind _color_johor (Variables|Color|GetColor_Johor))
  (bind _color_pahang (Variables|Color|GetColor_Pahang))
  (bind _color_melaka (Variables|Color|GetColor_Melaka))
  (bind _color_negerisembilan (Variables|Color|GetColor_NegeriSembilan))
  (bind _color_selangor (Variables|Color|GetColor_Selangor))
  (bind _color_putrajaya (Variables|Color|GetColor_Putrajaya))
  (bind _color_kualalumpur (Variables|Color|GetColor_KualaLumpur))
  (bind _color_perak (Variables|Color|GetColor_Perak))
  (bind _color_kelantan (Variables|Color|GetColor_Kelantan))
  (bind _color_terengganu (Variables|Color|GetColor_Terengganu))
  (bind _color_kedah (Variables|Color|GetColor_Kedah))
  (bind _color_penang (Variables|Color|GetColor_Penang))
  (bind _color_perlis (Variables|Color|GetColor_Perlis))
  (bind _color_sarawak (Variables|Color|GetColor_Sarawak))
  (bind _color_sabah (Variables|Color|GetColor_Sabah))
  (bind _color_labuan (Variables|Color|GetColor_Labuan))
  (Rendering|Material|SetVectorParameterValueonMaterials (Variables|Default|GetJohor) "Color" (Math|Vector|MakeVector (.r _color_johor) (.g _color_johor) (.b _color_johor)))
  (Rendering|Material|SetVectorParameterValueonMaterials (Variables|Default|GetPahang) "Color" (Math|Vector|MakeVector (.r _color_pahang) (.g _color_pahang) (.b _color_pahang)))
  (Rendering|Material|SetVectorParameterValueonMaterials (Variables|Default|GetMelaka) "Color" (Math|Vector|MakeVector (.r _color_melaka) (.g _color_melaka) (.b _color_melaka)))
  (Rendering|Material|SetVectorParameterValueonMaterials (Variables|Default|GetNegeriSembilan) "Color" (Math|Vector|MakeVector (.r _color_negerisembilan) (.g _color_negerisembilan) (.b _color_negerisembilan)))
  (Rendering|Material|SetVectorParameterValueonMaterials (Variables|Default|GetSelangor) "Color" (Math|Vector|MakeVector (.r _color_selangor) (.g _color_selangor) (.b _color_selangor)))
  (Rendering|Material|SetVectorParameterValueonMaterials (Variables|Default|GetPutrajaya) "Color" (Math|Vector|MakeVector (.r _color_putrajaya) (.g _color_putrajaya) (.b _color_putrajaya)))
  (Rendering|Material|SetVectorParameterValueonMaterials (Variables|Default|GetKualaLumpur) "Color" (Math|Vector|MakeVector (.r _color_kualalumpur) (.g _color_kualalumpur) (.b _color_kualalumpur)))
  (Rendering|Material|SetVectorParameterValueonMaterials (Variables|Default|GetPerak) "Color" (Math|Vector|MakeVector (.r _color_perak) (.g _color_perak) (.b _color_perak)))
  (Rendering|Material|SetVectorParameterValueonMaterials (Variables|Default|GetKelantan) "Color" (Math|Vector|MakeVector (.r _color_kelantan) (.g _color_kelantan) (.b _color_kelantan)))
  (Rendering|Material|SetVectorParameterValueonMaterials (Variables|Default|GetTerengganu) "Color" (Math|Vector|MakeVector (.r _color_terengganu) (.g _color_terengganu) (.b _color_terengganu)))
  (Rendering|Material|SetVectorParameterValueonMaterials (Variables|Default|GetKedah) "Color" (Math|Vector|MakeVector (.r _color_kedah) (.g _color_kedah) (.b _color_kedah)))
  (Rendering|Material|SetVectorParameterValueonMaterials (Variables|Default|GetPenang) "Color" (Math|Vector|MakeVector (.r _color_penang) (.g _color_penang) (.b _color_penang)))
  (Rendering|Material|SetVectorParameterValueonMaterials (Variables|Default|GetPerlis) "Color" (Math|Vector|MakeVector (.r _color_perlis) (.g _color_perlis) (.b _color_perlis)))
  (Rendering|Material|SetVectorParameterValueonMaterials (Variables|Default|GetSarawak) "Color" (Math|Vector|MakeVector (.r _color_sarawak) (.g _color_sarawak) (.b _color_sarawak)))
  (Rendering|Material|SetVectorParameterValueonMaterials (Variables|Default|GetSabah) "Color" (Math|Vector|MakeVector (.r _color_sabah) (.g _color_sabah) (.b _color_sabah)))
  (Rendering|Material|SetVectorParameterValueonMaterials (Variables|Default|GetLabuan) "Color" (Math|Vector|MakeVector (.r _color_labuan) (.g _color_labuan) (.b _color_labuan))))

(fn SetActiveState
  (params (State :type String))
  (Utilities|FlowControl|Sequence
    (:then_0
      (CallFunction|AssignDefaultMaterialtoStates)
      (switch string State
        (:Perlis
          (Rendering|Material|SetMaterial (Variables|Default|GetPerlis) 0 (Variables|Default|GetHighLightMaterial)))
        (:Kedah
          (Rendering|Material|SetMaterial (Variables|Default|GetKedah) 0 (Variables|Default|GetHighLightMaterial)))
        (:Kelantan
          (Rendering|Material|SetMaterial (Variables|Default|GetKelantan) 0 (Variables|Default|GetHighLightMaterial)))
        (:Terengganu
          (Rendering|Material|SetMaterial (Variables|Default|GetTerengganu) 0 (Variables|Default|GetHighLightMaterial)))
        (:Penang
          (Rendering|Material|SetMaterial (Variables|Default|GetPahang) 0 (Variables|Default|GetHighLightMaterial)))
        (:Perak
          (Rendering|Material|SetMaterial (Variables|Default|GetPerak) 0 (Variables|Default|GetHighLightMaterial)))
        (:Pahang
          (Rendering|Material|SetMaterial (Variables|Default|GetPahang) 0 (Variables|Default|GetHighLightMaterial)))
        (:Selangor
          (Rendering|Material|SetMaterial (Variables|Default|GetSelangor) 0 (Variables|Default|GetHighLightMaterial)))
        (:Kuala%20Lumpur
          (Rendering|Material|SetMaterial (Variables|Default|GetKualaLumpur) 0 (Variables|Default|GetHighLightMaterial)))
        (:Putrajaya
          (Rendering|Material|SetMaterial (Variables|Default|GetPutrajaya) 0 (Variables|Default|GetHighLightMaterial)))
        (:Negeri%20Sembilan
          (Rendering|Material|SetMaterial (Variables|Default|GetNegeriSembilan) 0 (Variables|Default|GetHighLightMaterial)))
        (:Melaka
          (Rendering|Material|SetMaterial (Variables|Default|GetMelaka) 0 (Variables|Default|GetHighLightMaterial)))
        (:Johor
          (Rendering|Material|SetMaterial (Variables|Default|GetJohor) 0 (Variables|Default|GetHighLightMaterial)))
        (:Labuan
          (Rendering|Material|SetMaterial (Variables|Default|GetLabuan) 0 (Variables|Default|GetHighLightMaterial)))
        (:Sabah
          (Rendering|Material|SetMaterial (Variables|Default|GetSabah) 0 (Variables|Default|GetHighLightMaterial)))
        (:Sarawak
          (Rendering|Material|SetMaterial (Variables|Default|GetSarawak) 0 (Variables|Default|GetHighLightMaterial)))))
    (:then_1
      (CallFunction|AssignColortoStates))))

(fn AssignDefaultMaterialtoStates
  (Utilities|FlowControl|Sequence
    (:then_0
      (Rendering|Material|SetMaterial (Variables|Default|GetPerlis) 0 (Variables|Default|GetDefaultMaterial)))
    (:then_1
      (Rendering|Material|SetMaterial (Variables|Default|GetKedah) 0 (Variables|Default|GetDefaultMaterial)))
    (:then_2
      (Rendering|Material|SetMaterial (Variables|Default|GetKelantan) 0 (Variables|Default|GetDefaultMaterial)))
    (:then_3
      (Rendering|Material|SetMaterial (Variables|Default|GetTerengganu) 0 (Variables|Default|GetDefaultMaterial)))
    (:then_4
      (Rendering|Material|SetMaterial (Variables|Default|GetPahang) 0 (Variables|Default|GetDefaultMaterial)))
    (:then_5
      (Rendering|Material|SetMaterial (Variables|Default|GetPerak) 0 (Variables|Default|GetDefaultMaterial)))
    (:then_6
      (Rendering|Material|SetMaterial (Variables|Default|GetPahang) 0 (Variables|Default|GetDefaultMaterial)))
    (:then_7
      (Rendering|Material|SetMaterial (Variables|Default|GetSelangor) 0 (Variables|Default|GetDefaultMaterial)))
    (:then_8
      (Rendering|Material|SetMaterial (Variables|Default|GetKualaLumpur) 0 (Variables|Default|GetDefaultMaterial)))
    (:then_9
      (Rendering|Material|SetMaterial (Variables|Default|GetPutrajaya) 0 (Variables|Default|GetDefaultMaterial)))
    (:then_10
      (Rendering|Material|SetMaterial (Variables|Default|GetNegeriSembilan) 0 (Variables|Default|GetDefaultMaterial)))
    (:then_11
      (Rendering|Material|SetMaterial (Variables|Default|GetMelaka) 0 (Variables|Default|GetDefaultMaterial)))
    (:then_12
      (Rendering|Material|SetMaterial (Variables|Default|GetJohor) 0 (Variables|Default|GetDefaultMaterial)))
    (:then_13
      (Rendering|Material|SetMaterial (Variables|Default|GetLabuan) 0 (Variables|Default|GetDefaultMaterial)))
    (:then_14
      (Rendering|Material|SetMaterial (Variables|Default|GetSabah) 0 (Variables|Default|GetDefaultMaterial)))
    (:then_15
      (Rendering|Material|SetMaterial (Variables|Default|GetSarawak) 0 (Variables|Default|GetDefaultMaterial)))))

(fn Zoomin
  (Math|Integer|IncrementInt (Variables|Default|GetCurrentZoomLevel)
    (:%20%20
      (Variables|Default|SetCurrentZoomLevel (Math|Integer|Clamp(Integer) (Variables|Default|GetCurrentZoomLevel) (Variables|Default|GetMinZoom) (Variables|Default|GetMaxZoom)))
      (CallFunction|UpdateZoom))))

(fn ZoomOut
  (Math|Integer|DecrementInt (Variables|Default|GetCurrentZoomLevel)
    (:%20%20
      (Variables|Default|SetCurrentZoomLevel (Math|Integer|Clamp(Integer) (Variables|Default|GetCurrentZoomLevel) (Variables|Default|GetMinZoom) (Variables|Default|GetMaxZoom)))
      (CallFunction|UpdateZoom))))

(fn UpdateZoom
  (switch int (Variables|Default|GetCurrentZoomLevel)
    (:0
      (bind _result (CallFunction|GetMapFocusDataWholeMalaysia))
      (Variables|Default|SetTargetFocusData _result))
    (:1
      (bind _result_2 (CallFunction|GetMapFocusDataHalfMalaysia))
      (Variables|Default|SetTargetFocusData _result_2))
    (:2
      (bind _result_3 (CallFunction|GetMapFocusDatabyStateName (Variables|Default|GetCurrentState)))
      (Variables|Default|SetTargetFocusData _result_3))))

(fn LoadMapFocusData
  (bind _outrownames (DataTable|GetDataTableRowNames "/Game/Data/MapFocusData.MapFocusData"))
  (for _array_element _outrownames
    (bind _returnvalue (Utilities|GetDataTableRow "/Game/Data/MapFocusData.MapFocusData" _array_element)
      (:then
        (Utilities|Array|Add (Variables|Default|GetMapFocusData) _returnvalue)))))

(fn GetMapFocusDataWholeMalaysia
  (return (Utilities|Array|Get(acopy) (Variables|Default|GetMapFocusData))))

(fn GetMapFocusDataHalfMalaysia
  (Utilities|FlowControl|Sequence
    (:then_0
      (for _array_element (Variables|Default|GetEastMalaysianState)
        (if (Utilities|Enum|Equal(Enum) _array_element (Variables|Default|GetCurrentState))
          (bind _result (CallFunction|GetMapFocusDatabyStateName "East"))
          (return _result))))
    (:then_1
      (bind _result_2 (CallFunction|GetMapFocusDatabyStateName "West"))
      (return _result_2))))

(fn GetMapFocusDatabyStateName
  (params (StateName :type String))
  (for _array_element (Variables|Default|GetMapFocusData)
    (if (Utilities|Enum|Equal(Enum) (.State (Utilities|Struct|BreakMapFocusStruct _array_element)) StateName)
      (return _array_element)))
  (return (Utilities|Array|Get(acopy) (Variables|Default|GetMapFocusData))))

(fn UpdateMapTransform
  (bind _returnvalue (Utilities|Time|GetWorldDeltaSeconds))
  (bind _self self)
  (bind _maptransformspeed (Variables|Default|GetMapTransformSpeed))
  (bind _targetfocusdata (Variables|Default|GetTargetFocusData))
  (bind _returnvalue_2 (Transformation|GetActorTransform _self))
  (bind _returnvalue_3 (* _returnvalue _maptransformspeed))
  (Transformation|SetActorLocation self (Math|Vector|Lerp(Vector) (.location _returnvalue_2) (.location (Variables|Default|GetTargetFocusData)) _returnvalue_3) false false)
  (Transformation|SetActorScale3D self (Math|Vector|Lerp(Vector) (.scale _returnvalue_2) (Math|Vector|MakeVector (.scale _targetfocusdata) 1.0 (.scale _targetfocusdata)) _returnvalue_3)))